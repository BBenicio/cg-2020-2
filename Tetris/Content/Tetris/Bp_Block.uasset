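; Tetris piece actor built from four block meshes, handling its own rotation and collision checks.
; BlockRotation cycles through 90-degree pitch steps up to MaxRotation, then restores the rotation from RotationRestore if the new pose collides.
; DetectCollision box-traces on Visibility from each mesh, either in place for rotation or one 100-unit cell down or sideways, stopping at the first hit.
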(event Custom|Block%20Rotation
  ;[0.04167 0.04167 0.04167] Rotate block
  (if (> (Variables|Default|GetMaxRotation) 0)
    (bind _result (Math|Integer|IncrementInt (Variables|Default|GetRotation))
      (:%20%20
        (if (> _result (Variables|Default|GetMaxRotation))
          (Variables|Default|SetRotation 0))
        (Transformation|SetActorRotation (Math|Rotator|MakeRotator 0.0 (Math|Conversions|ToFloat(Integer) (* (Variables|Default|GetRotation) 90)) 0.0))
        (bind _collided (CallFunction|DetectCollision true false false))
        (if _collided
          (Transformation|SetActorRotation (Math|Rotator|MakeRotator 0.0 (Math|Conversions|ToFloat(Integer) (Utilities|Array|Get(acopy) (Variables|Default|GetRotationRestore) (Variables|Default|GetRotation))) 0.0))
          (Math|Integer|DecrementInt (Variables|Default|GetRotation)))))))

(event EventBeginPlay
  ;[0.04167 0.04167 0.04167] Setup block array
  (Variables|Default|SetAllBlocks (Utilities|Array|MakeArray (Variables|Default|GetSm_Center) (Variables|Default|GetSm_01) (Variables|Default|GetSm_02) (Variables|Default|GetSm_03))))

(fn ConstructionScript)

(fn DetectCollision
  (params (Rotation :type Boolean) (Down :type Boolean) (Left :type Boolean))
  ;[0.04167 0.04167 0.04167] Set the vector depending on the option selected
  (if Rotation
    (LocalVariables|SetLocalLocation "0, 0, 0")
    (elif Down
      (LocalVariables|SetLocalLocation "0, 0,100.000000")
      (elif Left
        (LocalVariables|SetLocalLocation "100.000000, 0, 0")
        (else
          (LocalVariables|SetLocalLocation "-100.000000, 0, 0")))))
  (bind _array_element (Utilities|Array|ForEachLoopwithBreak (Variables|Default|GetAllBlocks) :!label _label)
    (:LoopBody
      (bind _returnvalue (Collision|BoxTraceByChannel (- (Transformation|GetWorldLocation _array_element) (LocalVariables|GetLocalLocation)) (+ (- (Transformation|GetWorldLocation _array_element) (LocalVariables|GetLocalLocation)) "0,40.000000, 0") "45.000000,20.000000,45.000000" "0, 0, 0" "TraceTypeQuery1" false 0 "None"))
      (if _returnvalue
        (goto _label Break)))
    (:Completed
      (return _returnvalue))))